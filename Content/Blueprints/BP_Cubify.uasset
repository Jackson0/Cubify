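; BP_Cubify voxelizes a referenced static mesh's surface into grid-snapped cubes, hiding the original mesh.
; BeginPlay caches LOD0 section 0's triangles in world space; Tick processes a few per frame.
; Larger triangles are lerp-scanned and send cubes to BP_CubeSpawnBroker; sub-grid ones only record a snapped centre.
; A location set and traces skip duplicates, plus cubes enclosed on six sides by overlapping cavity volumes.
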(event `self.ReceiveBeginPlay`
  (bind _staticmeshactor (`self.StaticMeshActor`))
  (bind _gridsize (`self.GridSize`))
  (bind _gridsize_2 (`self.GridSize`))
  (bind _gridsize_3 (`self.GridSize`))
  (bind _neighbourcubes (`self.NeighbourCubes`))
  (bind _returnvalue (/ (`self.GridSize`) 98.0))
  (`KismetSystemLibrary.Delay` 0.2)
  (`|ExecutionSequence`
    (:`then_0`
      ;[1 1 1] Spawn Cube Broker Actor
      (bind _returnvalue_2 (`GameplayStatics.GetActorOfClass` "/Game/Blueprints/BP_CubeSpawnBroker.BP_CubeSpawnBroker_C"))
      (set `self.CubeBroker` _returnvalue_2)
      ;[0.9264 1 0] Set scale of cubes...
      (set `self.CubeScale` (`KismetMathLibrary.MakeVector` _returnvalue _returnvalue _returnvalue)))
    (:`then_1`
      ;[1 0.3976 0.2168] Grab Location, Scale and Rotation
      (set `self.ActorRotation` (`self.K2_GetActorRotation` (`self.StaticMeshActor`)))
      (set `self.ActorScale` (`SceneComponent.K2_GetComponentScale` (`StaticMeshActor.StaticMeshComponent` (`self.StaticMeshActor`))))
      (set `self.Actor Location` (`SceneComponent.K2_GetComponentLocation` (`StaticMeshActor.StaticMeshComponent` (`self.StaticMeshActor`))))
      (set `self.SelfLocation` (`SceneComponent.K2_GetComponentLocation` (`self.DefaultSceneRoot`))))
    (:`then_2`
      ;[0 1 0.8633] Get the vertices and triangles
      (`SceneComponent.SetVisibility` (`StaticMeshActor.StaticMeshComponent` _staticmeshactor) false false)
      (bind (_vertices _triangles) (`KismetProceduralMeshLibrary.GetSectionFromStaticMesh` (`StaticMeshComponent.StaticMesh` (`StaticMeshActor.StaticMeshComponent` _staticmeshactor))))
      (bind _output_get (set `self.VerticesMainArray` _vertices))
      (set `self.Triangles` _triangles)
      (for (_array_element _array_index) _output_get
        (`KismetArrayLibrary.Array_Set` (`self.VerticesMainArray`) _array_index (+ (`KismetMathLibrary.GreaterGreater_VectorRotator` (* _array_element (`self.ActorScale`)) (`self.ActorRotation`)) (`self.Actor Location`))))
      (set `self.DoneWithInitial?` true))
    (:`then_3`
      ;[0.9935 1 0.3423] NeighbourCubes Location Setup
      ;;[1 1 1] Up & Down
      (`KismetArrayLibrary.Array_Add` _neighbourcubes (`KismetMathLibrary.MakeVector` 0.0 0.0 _gridsize_2))
      (`KismetArrayLibrary.Array_Add` _neighbourcubes (`KismetMathLibrary.MakeVector` 0.0 0.0 (- 0.0 _gridsize_2)))
      ;;[1 1 1] Left & Right
      (`KismetArrayLibrary.Array_Add` _neighbourcubes (`KismetMathLibrary.MakeVector` 0.0 _gridsize_3))
      (`KismetArrayLibrary.Array_Add` _neighbourcubes (`KismetMathLibrary.MakeVector` 0.0 (- 0.0 _gridsize_3)))
      ;;[1 1 1] Front & Back
      (`KismetArrayLibrary.Array_Add` _neighbourcubes (`KismetMathLibrary.MakeVector` _gridsize))
      (`KismetArrayLibrary.Array_Add` _neighbourcubes (`KismetMathLibrary.MakeVector` (- 0.0 _gridsize))))))

(event `self.ReceiveTick`
  (params (DeltaSeconds :type "Float (single-precision)"))
  (bind _middlelinesegmentscount (`self.MiddleLineSegmentsCount`))
  (bind _oppositecornervert (`self.OppositeCornerVert`))
  (bind _trianglestotal (`self.TrianglesTotal`))
  (bind _vertexsnappedtogrid (`self.VertexSnappedToGrid`))
  (bind _vertexsnappedtogrid_2 (`self.VertexSnappedToGrid`))
  (bind (_corner1 _corner2 _corner3) (`self.GetTrianglePoints` _trianglestotal))
  ;[1 0.08891 0.1786] Initial status checks
  (if (`self.DoneWithInitial?`)
    (if (not (`self.AllDone?`))
      (for _ (range 6)
        (if (> _trianglestotal (- (`KismetArrayLibrary.Array_Length` (`self.Triangles`)) 1))
          (set `self.AllDone?` true)
          (break)
          (else
            (bind _smallerthangridunit (`self.CheckSizeAgainstGrid` _corner1 _corner2 _corner3 (`self.GridSize`))
              (:`Exec_Out`
                (set `self.TrianglesTotal` (+ (`self.TrianglesTotal`) 3))
                (if _smallerthangridunit
                  ;[0.627 1 0.7768] If any triangle is smaller than the grid size, just spawn a cube in the middle of it.
                  (`BlueprintSetLibrary.Set_Add` (`self.CubeLocationSet`) (`KismetMathLibrary.Vector_SnappedToGrid` (`KismetMathLibrary.GetVectorArrayAverage` (`|MakeArray` _corner1 _corner2 _corner3)) (`self.GridSize`)))
                  (else
                    (bind (_longestsidevert_1 _longestsidevert_2) (`self.TriangleLongestSide`)
                      (:`Exec_Out`
                        ;[0.1337 1 0.737] Get the middle of the longest side of triangle
                        (bind _output_get (set `self.HypoMidPoint` (/ (+ _longestsidevert_1 _longestsidevert_2) 2.0)))
                        ;[0 0.3389 1] Use Lerp to go through points all along the 2 short sides of the triangle, between which we'll be plotting points where cubes need to be placed.
                        (set `self.MiddleLineSegmentsCount` (`KismetMathLibrary.FTrunc` (+ (/ (`KismetMathLibrary.Vector_Distance` _output_get (`self.OppositeCornerVert`)) (`self.GridSize`)) (`self.Scan Resolution`))))
                        (for _index (range (+ _middlelinesegmentscount 1))
                          (bind _returnvalue (* _index (/ 1.0 (`KismetMathLibrary.Conv_IntToDouble` _middlelinesegmentscount))))
                          (bind _output_get_2 (set `self.CubeScanLinePointA` (`KismetMathLibrary.VLerp` (`self.LongestSideVert_1`) _oppositecornervert _returnvalue)))
                          (bind _output_get_3 (set `self.CubeScanLinePointB` (`KismetMathLibrary.VLerp` (`self.LongestSideVert_2`) _oppositecornervert _returnvalue)))
                          ;[0 0.4112 1] Calculate how many cubes will fit between these 2 points...
                          (bind _output_get_4 (set `self.CubeLineScanSegmentLength(Sqr)` (`KismetMathLibrary.Vector_Distance` _output_get_2 _output_get_3)))
                          (bind _returnvalue_2 (/ _output_get_4 (`self.GridSize`)))
                          ;[0 0.4244 1] ..and using lerp again to finally get the location of every cube between those 2 points.
                          (for _index_2 (range (+ (`KismetMathLibrary.FTrunc` _returnvalue_2) 1))
                            ;[1 0 0.9362] Snap the location to specified cube grid size.
                            (set `self.VertexSnappedToGrid` (`KismetMathLibrary.Vector_SnappedToGrid` (`KismetMathLibrary.VLerp` (`self.CubeScanLinePointA`) (`self.CubeScanLinePointB`) (* _index_2 (/ 1.0 _returnvalue_2))) (`self.GridSize`)))
                            ;[1 1 1 1 15] Do I already have a cube here? (Check in my set-o-cubes)
                            (if (not (`BlueprintSetLibrary.Set_Contains` (`self.CubeLocationSet`) (`self.VertexSnappedToGrid`)))
                              ;[1 1 1] Did some other cubified mesh spawn a cube here already? Dont want duplicates...
                              (bind (_outhit _returnvalue_3) (`KismetSystemLibrary.LineTraceSingleForObjects` _vertexsnappedtogrid (+ _vertexsnappedtogrid (1.0 1.0 1.0)) (`self.Object Type Cube`)))
                              (if (not _returnvalue_3)
                                ;[1 1 1 1 12] Is this cube position overlapping more than just my own collision shape? If yes, we might not want to spawn a cube here as we might be inside a collective cavity space. More tests to follow...
                                (bind _outhits (`KismetSystemLibrary.BoxTraceMultiForObjects` :`Start` _vertexsnappedtogrid_2 :`End` _vertexsnappedtogrid_2 :`HalfSize` (`KismetMathLibrary.Conv_DoubleToVector` (* (`self.GridSize`) 0.4)) :`ObjectTypes` (`self.Object Type Cavity`) :`bIgnoreSelf` false :`DrawTime` 50.0))
                                (if (> (`KismetArrayLibrary.Array_Length` _outhits) 1)
                                  ;[1 1 1] Check all around this cube. If it is found to be surrounded by "cavity space" on all 6 sides, we don't want to spawn it
                                  (set `self.NeighbourCubeCount` 0)
                                  (for _array_element (`self.NeighbourCubes`)
                                    (bind _returnvalue_4 (+ (`self.VertexSnappedToGrid`) _array_element))
                                    (bind (_outhit_2 _returnvalue_5) (`KismetSystemLibrary.LineTraceSingleForObjects` :`Start` _returnvalue_4 :`End` (+ _returnvalue_4 (1.0 1.0 1.0)) :`ObjectTypes` (`self.Object Type Cavity`) :`bIgnoreSelf` false :`DrawTime` 10.0))
                                    (if _returnvalue_5
                                      (`/Engine/EditorBlueprintResources/StandardMacros.IncrementInt` (`self.NeighbourCubeCount`))))
                                  (if (not (== (`self.NeighbourCubeCount`) 6))
                                    ;[0.1072 1 0] Add Cube
                                    (`BlueprintSetLibrary.Set_Add` (`self.CubeLocationSet`) (`self.VertexSnappedToGrid`) :!label _label)
                                    (`/Game/Blueprints/BP_CubeSpawnBroker.Add Cube` (`self.CubeBroker`) (- (`self.VertexSnappedToGrid`) (`self.SelfLocation`)) (`self.CubeScale`)))
                                  (else
                                    (goto _label)))))))))))))))))))

(fn `UserConstructionScript`)