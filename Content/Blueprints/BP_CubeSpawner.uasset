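; BP_CubeSpawner renders one area's cubes as instanced static meshes in a cubify system where the player shoots cubes away.
; A randomly offset looping timer removes flagged instances and spawns the set difference between its locations object and already spawned cubes.
; KillCube records hit cubes in a global cavity set.
; It line-traces their six neighbours, asking CubeSpawnBroker to add cubes in empty non-cavity spots, so the cube volume expands around holes.
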(event `self.ReceiveBeginPlay`
  (bind _gridsize (`self.GridSize`))
  (bind _gridsize_2 (`self.GridSize`))
  (bind _gridsize_3 (`self.GridSize`))
  (bind _neighbourcubes (`self.NeighbourCubes`))
  (`KismetSystemLibrary.Delay` 0.0)
  (`|ExecutionSequence`
    (:`then_0`
      ;[0 1 0.4638] Grab some values from "BP_CubeSystemInit" (Grid size and Object "Global Cavity Object" into which all destroyed cubes locations will be stored.)
      (bind _returnvalue (`GameplayStatics.GetActorOfClass` "/Game/Blueprints/BP_CubeSystemINIT.BP_CubeSystemINIT_C"))
      (set `self.GridSize` (`/Game/Blueprints/BP_CubeSystemINIT.CubeGridSize` _returnvalue))
      (set `self.Global Cavity Object` (`/Game/Blueprints/BP_CubeSystemINIT.GlobalCavityObject` _returnvalue)))
    (:`then_1`
      ;[0.9935 1 0.3423] Create a array with coordinates corresponding to a cube's "neighbours".
      ;;[1 1 1] Up & Down
      (`KismetArrayLibrary.Array_Add` _neighbourcubes (`KismetMathLibrary.MakeVector` 0.0 0.0 _gridsize_2))
      (`KismetArrayLibrary.Array_Add` _neighbourcubes (`KismetMathLibrary.MakeVector` 0.0 0.0 (- 0.0 _gridsize_2)))
      ;;[1 1 1] Left & Right
      (`KismetArrayLibrary.Array_Add` _neighbourcubes (`KismetMathLibrary.MakeVector` 0.0 _gridsize_3))
      (`KismetArrayLibrary.Array_Add` _neighbourcubes (`KismetMathLibrary.MakeVector` 0.0 (- 0.0 _gridsize_3)))
      ;;[1 1 1] Front & Back
      (`KismetArrayLibrary.Array_Add` _neighbourcubes (`KismetMathLibrary.MakeVector` _gridsize))
      (`KismetArrayLibrary.Array_Add` _neighbourcubes (`KismetMathLibrary.MakeVector` (- 0.0 _gridsize))))
    (:`then_2`
      ;[1 0.4552 0.08618] Get this actor's world location for use in new cube location calulation
      (set `self.MyWorldLocation` (`SceneComponent.K2_GetComponentLocation` (`self.DefaultSceneRoot`))))
    (:`then_3`
      ;[0.7098 1 0] Get Cube Scale value
      (set `self.Cube Scale` (`/Game/Blueprints/BP_CubeLocations.CubeScale` (`self.MyCubeLocationsObject`))))
    (:`then_4`
      ;[0 1 0.4575] Set main loop timer up with unique offset
      (`KismetSystemLibrary.K2_SetTimerDelegate` (delegate `LightMeUp`) (`KismetMathLibrary.RandomFloatInRange` 0.01 0.1) true))))

(event `LightMeUp`
  (bind _mycubelocationsobject (`self.MyCubeLocationsObject`))
  ;[0 1 0.4575] Set main loop timer up with unique offset
  ;[0 1 0.8882] Check if "Kill Cube" function has been called, ie a cube has been hit/shot by player.
  (if (`self.bGotCubesToRemove?`)
    ;[0 0.8194 1] Get cubes in area around hit cube, remove them.
    (set `self.bGotCubesToRemove?` false)
    (for _array_element (`InstancedStaticMeshComponent.GetInstancesOverlappingSphere` (`self.InstancedStaticMesh`) (`self.InstanceOverlapSphereLocation`) 150.0 true)
      (`InstancedStaticMeshComponent.RemoveInstance` (`self.InstancedStaticMesh`) _array_element)))
  ;[0 1 0.9513] If "BP_CubeSpawnBroker" has added new cubes to "Cubes Locations Object" associated with this spawner (either in initial mesh cubify process or because of expanding cubes after player shot some) ,compare the set of all cubes that should be in this spawner's area, with the set of cubes already spawned. We need to spawn the difference.
  (if (`/Game/Blueprints/BP_CubeLocations.NewCubesAdded?` _mycubelocationsobject)
    (set `/Game/Blueprints/BP_CubeLocations.NewCubesAdded?` false _mycubelocationsobject)
    (set `self.CubesToSpawn` (`/Game/Blueprints/BP_CubeLocations.CubeVectorSet` _mycubelocationsobject))
    (bind _result (`BlueprintSetLibrary.Set_Difference` (`self.CubesToSpawn`) (`self.CubesAlreadySpawned`)))
    (bind _output_get (set `self.DifferenceSet` _result))
    ;[0 1 0.9668] If there are some cubes in the difference set, put them all in an array to be processed.
    (if (> (`BlueprintSetLibrary.Set_Length` _output_get) 0)
      (bind _result_2 (`BlueprintSetLibrary.Set_Union` (`self.CubesAlreadySpawned`) (`self.CubesToSpawn`)))
      (set `self.CubesAlreadySpawned` _result_2)
      (bind _result_3 (`BlueprintSetLibrary.Set_ToArray` _output_get))
      ;[0 0.4508 1] Add instances to ISM
      (for _array_element_2 _result_3
        (`KismetArrayLibrary.Array_Add` (`self.Instance Transforms`) (`KismetMathLibrary.MakeTransform` (- _array_element_2 (`self.MyWorldLocation`)) (struct) (`self.Cube Scale`)))
        (`InstancedStaticMeshComponent.AddInstances` (`self.InstancedStaticMesh`) (`self.Instance Transforms`) false)
        (`KismetArrayLibrary.Array_Clear` (`self.Instance Transforms`))))))

(fn `KillCube`
  (params (Location :type "Vector Structure"))
  (locals (CurrentIndex :type Integer) (CubeToKill :type "Vector Structure"))
  ;[0 1 0.2231] Called from "BP_FirstPersonCharacterCubify", along with hit location.
  (bind _output_get (set `self.InstanceOverlapSphereLocation` Location))
  ;[0 1 0.7594] Get cube instances in Sphere Overlap
  (set `self.bGotCubesToRemove?` true)
  (for _array_element (`InstancedStaticMeshComponent.GetInstancesOverlappingSphere` (`self.InstancedStaticMesh`) _output_get 150.0 true)
    ;[0 0.6944 1] Remove these instances from "CubeLocationsObject" set and from "Cubes to Spawn" set
    (bind _output_get_2 (set `local.CurrentIndex` _array_element))
    (bind _output_get_3 (set `local.CubeToKill` (.location (`InstancedStaticMeshComponent.GetInstanceTransform` (`self.InstancedStaticMesh`) _output_get_2 true))))
    (`BlueprintSetLibrary.Set_Remove` (`/Game/Blueprints/BP_CubeLocations.CubeVectorSet` (`self.MyCubeLocationsObject`)) _output_get_3)
    (`BlueprintSetLibrary.Set_Remove` (`self.CubesToSpawn`) _output_get_3)
    ;[1 0.4674 0] Check around each cube that's set to be removed. If cube is surrounded by "Cavity space" or other cubes, simply remove. If cube is neighbouring any open space, a new cube needs to be spawned in order to expand the area of cubes.
    (for _array_element_2 (`self.NeighbourCubes`)
      (bind _returnvalue (+ _array_element_2 (`local.CubeToKill`)))
      (if (not (`BlueprintSetLibrary.Set_Contains` (`/Game/Blueprints/BP_GlobalCavityObject.GlobalCavitySet` (`self.Global Cavity Object`)) _returnvalue))
        (bind (_outhit _returnvalue_2) (`KismetSystemLibrary.LineTraceSingleForObjects` :`Start` _returnvalue :`End` (+ _returnvalue (0.2 0.2 0.2)) :`ObjectTypes` (`self.Object Types`) :`bIgnoreSelf` false))
        (if (not _returnvalue_2)
          (`/Game/Blueprints/BP_CubeSpawnBroker.Add Cube` (`self.CubeSpawnBroker`) _returnvalue (`self.Cube Scale`)))))
    (`BlueprintSetLibrary.Set_Add` (`/Game/Blueprints/BP_GlobalCavityObject.GlobalCavitySet` (`self.Global Cavity Object`)) _output_get_3)))

(fn `UserConstructionScript`)