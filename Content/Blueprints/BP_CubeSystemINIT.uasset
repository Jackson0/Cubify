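; Singleton initializer for the cube system that converts "Cavity" collision static mesh actors into cubes.
; After a short delay it spawns a BP_CubeSpawnBroker, creates a global object for destroyed-cube positions, and gathers those actors.
; A selection sort orders them nearest-to-player first.
; Tick then feeds them to temporary BP_Cubify actors one at a time, destroying each when finished and printing progress.
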(event `self.ReceiveBeginPlay`
  (bind _currentsmallestsma (`self.CurrentSmallestSMA`))
  (bind _returnvalue (`SceneComponent.K2_GetComponentLocation` (`Character.CapsuleComponent` (`GameplayStatics.GetPlayerCharacter` 0))))
  (`KismetSystemLibrary.Delay` 2.0)
  ;[1 0 0] Ensure only one instance of this class
  (bind _outactors (`GameplayStatics.GetAllActorsOfClass` "BP_CubeSystemINIT_C"))
  (if (> (`KismetArrayLibrary.Array_Length` _outactors) 1)
    (`KismetSystemLibrary.PrintString` "Error: ONLY 1 INIT ALLOWED" true true (struct :`R` 1.0 :`B` 0.009094 :`A` 1.0) 120.0)
    (else
      (`|ExecutionSequence`
        (:`then_0`
          (set `self.CubeInstanceSectionSize` (* (`self.CubeInstanceSectionSize`) (`self.CubeGridSize`))))
        (:`then_1`
          (bind _returnvalue_2 (`|SpawnActorFromClass` "/Game/Blueprints/BP_CubeSpawnBroker.BP_CubeSpawnBroker_C" (`KismetMathLibrary.MakeTransform` (`SceneComponent.K2_GetComponentLocation` (`self.DefaultSceneRoot`))) "Undefined" "OverrideRootScale" null null))
          (set `/Game/Blueprints/BP_CubeSpawnBroker.CubeInstanceSectionSize` (`self.CubeInstanceSectionSize`) _returnvalue_2))
        (:`then_2`
          ;[1 0.5069 0] Collect all the static mesh actors with "Cavity" collision object type
          (bind _outactors_2 (`GameplayStatics.GetAllActorsOfClass` "/Script/Engine.StaticMeshActor"))
          (for _array_element _outactors_2
            (if (`|EnumEquality` (`PrimitiveComponent.GetCollisionObjectType` (`StaticMeshActor.StaticMeshComponent` _array_element)) "ECC_GameTraceChannel2")
              (`KismetArrayLibrary.Array_Add` (`self.AllSMA's`) _array_element))))
        (:`then_3`
          ;[1 1 1] Create the object that will store positions of all destroyed cubes (so we know where not to spawn new cubes)
          (bind _returnvalue_3 (`|GenericCreateObject` "/Game/Blueprints/BP_GlobalCavityObject.BP_GlobalCavityObject_C" self))
          (set `self.GlobalCavityObject` _returnvalue_3))
        (:`then_4`
          ;[0 1 0.6707] Sort static mesh actors by distance from player... we want the ones nearest to the player to be "cubified" first
          (set `self.SMA_Array_Count` (- (`KismetArrayLibrary.Array_Length` (`self.AllSMA's`)) 1))
          (while (`self.bStillBusySorting?`)
            (set `self.CurrentSmallestSMA` (`|GetArrayItem` (`self.AllSMA's`)))
            (for _array_element_2 (`self.AllSMA's`)
              (if (< (`KismetMathLibrary.Vector_Distance` (`SceneComponent.K2_GetComponentLocation` (`StaticMeshActor.StaticMeshComponent` _array_element_2)) _returnvalue) (`KismetMathLibrary.Vector_Distance` _returnvalue (`SceneComponent.K2_GetComponentLocation` (`StaticMeshActor.StaticMeshComponent` (`self.CurrentSmallestSMA`)))))
                (set `self.CurrentSmallestSMA` _array_element_2)))
            (`KismetArrayLibrary.Array_Add` (`self.AllSMA'sTemp`) _currentsmallestsma)
            (`KismetArrayLibrary.Array_RemoveItem` (`self.AllSMA's`) _currentsmallestsma)
            (if (== (`KismetArrayLibrary.Array_Length` (`self.AllSMA's`)) 0)
              (set `self.bStillBusySorting?` false)
              (set `self.AllSMA's` (`self.AllSMA'sTemp`))))
          (set `self.ProsessedCounter` 0))))))

(event `self.ReceiveTick`
  (params (DeltaSeconds :type "Float (single-precision)"))
  (bind _prosessedcounter (`self.ProsessedCounter`))
  (bind _sma_array_count (`self.SMA_Array_Count`))
  ;[0 1 0.25] Process all static meshes
  (if (`self.bStillBusySorting?`)
    _
    (elif (`self.bAllSpawningDone?`)
      _
      (elif (`self.bCurrentSpawnDone?`)
        (bind _returnvalue (`|SpawnActorFromClass` "/Game/Blueprints/BP_Cubify.BP_Cubify_C" (`KismetMathLibrary.MakeTransform` (0.0 0.0 0.0)) "Undefined" "OverrideRootScale" null null))
        (set `self.CurrentCubify` _returnvalue)
        (set `/Game/Blueprints/BP_Cubify.StaticMeshActor` (`|GetArrayItem` (`self.AllSMA's`) (`self.ProsessedCounter`)) (`self.CurrentCubify`))
        (set `/Game/Blueprints/BP_Cubify.GridSize` (`self.CubeGridSize`) (`self.CurrentCubify`))
        (set `/Game/Blueprints/BP_Cubify.Scan Resolution` (`self.Scan Resolution`) (`self.CurrentCubify`))
        (set `self.bCurrentSpawnDone?` false)
        (elif (`/Game/Blueprints/BP_Cubify.AllDone?` (`self.CurrentCubify`))
          (set `self.bCurrentSpawnDone?` true)
          (`self.K2_DestroyActor` (`self.CurrentCubify`))
          (`/Engine/EditorBlueprintResources/StandardMacros.IncrementInt` _prosessedcounter
            (:`  `
              (if (> _prosessedcounter _sma_array_count)
                (set `self.bAllSpawningDone?` true)
                (else
                  (`KismetSystemLibrary.PrintString` (`KismetStringLibrary.Concat_StrStr` (`KismetStringLibrary.Conv_IntToString` _prosessedcounter) " of " (`KismetStringLibrary.Conv_IntToString` _sma_array_count) " done...") true true (struct :`R` 0.002067 :`B` 1.0 :`A` 1.0)))))))))))

(fn `UserConstructionScript`)