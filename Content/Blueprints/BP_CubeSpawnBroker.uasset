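; BP_CubeSpawnBroker manages which regions of cubes have live BP_CubeSpawner actors near the player.
; AddCube snaps positions to a section grid and stores them in a map of per-section BP_CubeLocations objects, flagging existing sections as changed.
; A looping timer compares each section to the player's distance, spawning a linked spawner within the render range from BP_CubeSystemINIT and destroying it beyond.
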(event `self.ReceiveBeginPlay`
  (`|ExecutionSequence`
    (:`then_0`
      ;[0 0.5712 1 1 14] Get the max render distance value from SystemINIT. This value will be used to determine if we should spawn (or destroy) a Cube Spawner Actor.
      (bind _returnvalue (`GameplayStatics.GetActorOfClass` "/Game/Blueprints/BP_CubeSystemINIT.BP_CubeSystemINIT_C"))
      (set `self.Cube Max Render Distance` (`/Game/Blueprints/BP_CubeSystemINIT.CubeMaxRenderDistance` _returnvalue)))
    (:`then_1`
      ;[0 1 0.4963] Go through the entire list of world locations where we need "BP_CubeSpawners".
      (`KismetSystemLibrary.K2_SetTimerDelegate` (delegate `Check distances`) 0.5 true))))

(event `Check distances`
  (bind _value (`BlueprintMapLibrary.Map_Find` (`self.CubeSpawnerLocations`) (`self.Current Key`)))
  (bind _myspawner (`/Game/Blueprints/BP_CubeLocations.MySpawner` (`BlueprintMapLibrary.Map_Find` (`self.CubeSpawnerLocations`) (`self.Current Key`))))
  ;[0 1 0.4963] Go through the entire list of world locations where we need "BP_CubeSpawners".
  (bind _keys (`BlueprintMapLibrary.Map_Keys` (`self.CubeSpawnerLocations`)))
  (for _array_element _keys
    (set `self.Current Key` _array_element)
    ;[0 0.6928 1] Compare this world location with player current location, and see if distance value between them is within "Cube Max Render Distance"
    (if (< (`KismetMathLibrary.Vector_Distance` (`SceneComponent.K2_GetComponentLocation` (`Character.CapsuleComponent` (`GameplayStatics.GetPlayerCharacter` 0))) (`self.Current Key`)) (`self.Cube Max Render Distance`))
      ;[0.1594 0.03282 1] If location where we need a Cube Spawner is within "Cube Max Render Distance", check first whether we don't already have a BP_CubeSpawner there. If not, go ahead and spawn one.
      (`/Engine/EditorBlueprintResources/StandardMacros.IsValid` (`/Game/Blueprints/BP_CubeLocations.MySpawner` _value)
        (:`Is Not Valid`
          (bind _returnvalue (`|SpawnActorFromClass` "/Game/Blueprints/BP_CubeSpawner.BP_CubeSpawner_C" (`KismetMathLibrary.MakeTransform` (0.0 0.0 0.0)) "Undefined" "OverrideRootScale" null null))
          (set `/Game/Blueprints/BP_CubeLocations.MySpawner` _returnvalue _value)
          (set `/Game/Blueprints/BP_CubeSpawner.MyCubeLocationsObject` _value _returnvalue)
          (set `/Game/Blueprints/BP_CubeLocations.NewCubesAdded?` true _value)
          (set `/Game/Blueprints/BP_CubeSpawner.CubeSpawnBroker` self _returnvalue)))
      (else
        ;[1 0.02322 0.1429] If distance exceeds "Cube Max Render Distance", and we DO have a BP_CubeSpawner there, destroy it.
        (`/Engine/EditorBlueprintResources/StandardMacros.IsValid` _myspawner
          (:`Is Valid`
            (`self.K2_DestroyActor` _myspawner)))))))

(fn `Add Cube`
  (params (CubeWorldLocation :type "Vector Structure") (CubeScale :type "Vector Structure"))
  (locals (CubeLocationSnapped :type "Vector Structure") (Cube_Location :type "Vector Structure") (Cube_Scale :type "Vector Structure"))
  (bind _value (`BlueprintMapLibrary.Map_Find` (`self.CubeSpawnerLocations`) (`local.CubeLocationSnapped`)))
  (set `local.Cube_Location` CubeWorldLocation)
  (set `local.Cube_Scale` CubeScale)
  ;[0.9673 1 0.2732] Snap the cube location received to grid and against a map of vectors, to see if it lies within an area where we already have a Cube Spawner actor servicing that area.
  (bind _output_get (set `local.CubeLocationSnapped` (`KismetMathLibrary.Vector_SnappedToGrid` (`local.Cube_Location`) (`self.CubeInstanceSectionSize`))))
  (if (`BlueprintMapLibrary.Map_Contains` (`self.CubeSpawnerLocations`) _output_get)
    ;[0 0.8662 1] If we do have a spawner in the area where we need a cube, add this cube's location to the BP_CubeLocations object mapped to the cube location vector.
    (set `/Game/Blueprints/BP_CubeLocations.NewCubesAdded?` true _value)
    (`BlueprintSetLibrary.Set_Add` (`/Game/Blueprints/BP_CubeLocations.CubeVectorSet` _value) (`local.Cube_Location`))
    (else
      ;[1 0.3701 0] If we don't have a spawner in the area where we need a cube, add to the map the location where we need a spawner, and map to that a BP_CubeLocations object. Add the cube location vector to this object.
      (bind _returnvalue (`|GenericCreateObject` "/Game/Blueprints/BP_CubeLocations.BP_CubeLocations_C" self))
      (`BlueprintSetLibrary.Set_Add` (`/Game/Blueprints/BP_CubeLocations.CubeVectorSet` _returnvalue) (`local.Cube_Location`))
      (set `/Game/Blueprints/BP_CubeLocations.CubeScale` (`local.Cube_Scale`) _returnvalue)
      (`BlueprintMapLibrary.Map_Add` (`self.CubeSpawnerLocations`) (`local.CubeLocationSnapped`) _returnvalue))))

(fn `UserConstructionScript`)